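; Enemy spawner that runs escalating waves of BP_NPC, placed in a row along X from its location.
; Destroyed and surviving enemies report back and leave the tracked list; survivors also increment LeftEnemies, which is never reset here.
; An emptied list triggers a delay, grows the total by a percentage, spawns the next wave plus LeftEnemies, then gives BP_Ship a heart.
; BeginPlay is empty, so nothing here starts the first wave.
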(event `self.ReceiveBeginPlay`)

(event `EndWave`
  (`KismetSystemLibrary.Delay` (`self.WaveDelay`))
  (set `self.TotalEnemies` (+ (`KismetMathLibrary.Round` (* (`self.AddPercentage`) (`self.TotalEnemies`))) (`self.TotalEnemies`)))
  (bind _result (`/Engine/EditorBlueprintResources/StandardMacros.IncrementInt` (`self.WaveIndex`))
    (:`  `
      (set `self.WaveIndex` _result)
      (`self.SpawnWave`)
      (bind _returnvalue (`GameplayStatics.GetActorOfClass` "/Game/Blueprints/BP_Ship.BP_Ship_C"))
      (`/Game/Blueprints/BP_Ship.AddHeart` _returnvalue))))

(fn `NotifyEnemyAlived`
  (params (Enemy :type "Actor Object Reference"))
  (bind _currentwaveenemies (`self.CurrentWaveEnemies`))
  (if (`KismetArrayLibrary.Array_Contains` (`self.CurrentWaveEnemies`) Enemy)
    (bind _result (`/Engine/EditorBlueprintResources/StandardMacros.IncrementInt` (`self.LeftEnemies`))
      (:`  `
        (set `self.LeftEnemies` _result)
        (`KismetArrayLibrary.Array_RemoveItem` _currentwaveenemies Enemy)
        (if (== (`KismetArrayLibrary.Array_Length` _currentwaveenemies) 0)
          (`self.EndWave`))))))

(fn `NotifyEnemyDestroyed`
  (params (Enemy :type "Actor Object Reference"))
  (bind _currentwaveenemies (`self.CurrentWaveEnemies`))
  (if (`KismetArrayLibrary.Array_Contains` (`self.CurrentWaveEnemies`) Enemy)
    (`KismetArrayLibrary.Array_RemoveItem` _currentwaveenemies Enemy)
    (if (== (`KismetArrayLibrary.Array_Length` _currentwaveenemies) 0)
      (`self.EndWave`))))

(fn `SpawnWave`
  (bind _returnvalue_x (`KismetMathLibrary.BreakVector` (`self.K2_GetActorLocation`)))
  (`KismetArrayLibrary.Array_Clear` (`self.CurrentWaveEnemies`))
  (if (> (`self.LeftEnemies`) 0)
    (set `self.TotalEnemies` (+ (`self.LeftEnemies`) (`self.TotalEnemies`))))
  (for _index (range 1 (+ (`self.TotalEnemies`) 1))
    (bind _returnvalue (`|SpawnActorFromClass` "/Game/Blueprints/BP_NPC.BP_NPC_C" (`KismetMathLibrary.MakeTransform` (`KismetMathLibrary.MakeVector` (+ (* _index (`self.Spacing X`)) _returnvalue_x))) "Undefined" "MultiplyWithRoot" null null))
    (`KismetArrayLibrary.Array_AddUnique` (`self.CurrentWaveEnemies`) _returnvalue)))

(fn `UserConstructionScript`)