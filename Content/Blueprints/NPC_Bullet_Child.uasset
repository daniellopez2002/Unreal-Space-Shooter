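; NPC_Bullet_Child is a projectile actor, apparently for NPC fire, that explodes and destroys itself on impact.
; When its Box component registers a hit, it spawns a side explosion particle at the hit location, plays a non-spatialized 2D explosion sound and removes the actor.
; The construction script defers to the parent, and this graph applies no damage and adds no movement logic.
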(event `self.Box.OnComponentHit`
  (params (HitComponent :type "PrimitiveComponent Object Reference") (OtherActor :type "Actor Object Reference") (OtherComp :type "PrimitiveComponent Object Reference") (NormalImpulse :type "Vector Structure") (Hit :type "HitResult Structure (by ref)"))
  (`GameplayStatics.SpawnEmitterAtLocation` "/Game/Realistic_Starter_VFX_Pack_Vol2/Particles/Explosion/P_Explosion_Side.P_Explosion_Side" (`.Location` (`GameplayStatics.BreakHitResult` Hit)))
  (`GameplayStatics.PlaySound2D` "/Game/Sounds/SFX/Esplosion_sfx.Esplosion_sfx" 1.0 1.0 0.0 null null)
  (`self.K2_DestroyActor`))

(fn `UserConstructionScript`
  (`parent.UserConstructionScript`))