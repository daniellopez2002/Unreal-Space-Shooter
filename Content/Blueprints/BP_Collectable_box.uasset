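; Collectable box actor that drifts along negative world X while rolling, and breaks apart on impact.
; BeginPlay picks a random roll rate, and Tick applies it alongside a swept move driven by Speed.
; Any hit on the Box component spawns an enlarged wood destruction particle effect and destroys the actor, with no pickup or reward logic.
; The actor also destroys itself once it passes a fixed negative X limit.
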(event `self.ReceiveBeginPlay`
  (set `self.RotationSpeed` (`KismetMathLibrary.RandomIntegerInRange` 5 15)))

(event `self.ReceiveTick`
  (params (DeltaSeconds :type "Float (single-precision)"))
  (bind (_returnvalue_x _returnvalue_y _returnvalue_z) (`KismetMathLibrary.BreakVector` (`self.K2_GetActorLocation`)))
  (bind (_returnvalue_roll _returnvalue_pitch _returnvalue_yaw) (`KismetMathLibrary.BreakRotator` (`self.K2_GetActorRotation`)))
  (bind _returnvalue_x_2 (`KismetMathLibrary.BreakVector` (`self.K2_GetActorLocation`)))
  (`self.K2_SetActorLocation` (`KismetMathLibrary.MakeVector` (- _returnvalue_x (* DeltaSeconds (`self.Speed `))) _returnvalue_y _returnvalue_z) true)
  (`self.K2_SetActorRotation` (`KismetMathLibrary.MakeRotator` (+ _returnvalue_roll (* DeltaSeconds (`self.RotationSpeed`)))))
  (if (<= _returnvalue_x_2 -4000.0)
    (`self.K2_DestroyActor`)))

(event `self.Box.OnComponentHit`
  (params (HitComponent :type "PrimitiveComponent Object Reference") (OtherActor :type "Actor Object Reference") (OtherComp :type "PrimitiveComponent Object Reference") (NormalImpulse :type "Vector Structure") (Hit :type "HitResult Structure (by ref)"))
  (`GameplayStatics.SpawnEmitterAtLocation` "/Game/Realistic_Starter_VFX_Pack_Vol2/Particles/Destruction/P_Destruction_Wood.P_Destruction_Wood" (`.Location` (`GameplayStatics.BreakHitResult` Hit)) (struct) (10.0 10.0 10.0))
  (`self.K2_DestroyActor`))

(fn `UserConstructionScript`)