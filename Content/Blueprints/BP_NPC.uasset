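; Enemy ship NPC driven by a Tick state machine: it flies in along -X without collision, then weaves on a sine wave with randomized phase.
; A looping timer starts on entering ZigZag and fires three bullets per volley until retreat.
; Past MinX it turns, shifts Y and speeds back out, notifying BP_EnemySpawner that it survived.
; Box hits explode it and report the kill; the Dead state only explodes and destroys it.
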(event `self.ReceiveBeginPlay`
  (`|ExecutionSequence`
    (:`then_0`
      (set `self.InverseOccilation` (`KismetMathLibrary.RandomBool`))
      (set `self.IsRetreat` false))
    (:`then_1`
      (`self.K2_SetActorRotation` (struct :`Yaw` 180.0))
      (bind _returnvalue (`GameplayStatics.GetActorOfClass` "/Game/Blueprints/BP_EnemySpawner.BP_EnemySpawner_C"))
      (set `self.Spawner` _returnvalue))))

(event `self.ReceiveTick`
  (params (DeltaSeconds :type "Float (single-precision)"))
  (bind _returnvalue_x (`KismetMathLibrary.BreakVector` (`self.K2_GetActorLocation`)))
  (bind (_returnvalue_x_2 _returnvalue_y) (`KismetMathLibrary.BreakVector` (`self.K2_GetActorLocation`)))
  (bind _returnvalue_x_3 (`KismetMathLibrary.BreakVector` (`self.K2_GetActorLocation`)))
  (bind _returnvalue_x_4 (`KismetMathLibrary.BreakVector` (`self.K2_GetActorLocation`)))
  (bind _returnvalue_x_5 (`KismetMathLibrary.BreakVector` (`self.K2_GetActorLocation`)))
  (bind (_returnvalue_x_6 _returnvalue_y_2 _returnvalue_z) (`KismetMathLibrary.BreakVector` (`self.K2_GetActorLocation`)))
  (bind _retreatyposition (`self.RetreatYPosition`))
  (bind _returnvalue (- _returnvalue_x_3 (* (`self.Speed`) DeltaSeconds)))
  (bind _returnvalue_2 (* (`self.Amplitude`) (`KismetMathLibrary.Sin` (* (`GameplayStatics.GetTimeSeconds`) (`self.Frequency`)))))
  (switch `/Game/Enum/EEnemyState` (`self.EnemyState`)
    (:`NewEnumerator0`
      (`PrimitiveComponent.SetCollisionEnabled` (`self.Box`) "NoCollision")
      (`self.K2_SetActorLocation` (`KismetMathLibrary.MakeVector` (- _returnvalue_x_3 (* (`self.Speed`) DeltaSeconds))) true)
      (if (<= _returnvalue_x (`self.TargetX`))
        (set `self.EnemyState` "NewEnumerator1")
        (`KismetSystemLibrary.K2_SetTimer` null "Fire" (`self.ShootRate`) true)))
    (:`NewEnumerator1`
      (`PrimitiveComponent.SetCollisionEnabled` (`self.Box`) "QueryAndPhysics")
      (if (`self.InverseOccilation`)
        (`self.K2_SetActorLocation` (`KismetMathLibrary.MakeVector` _returnvalue _returnvalue_2) true)
        (else
          (bind _result (`/Engine/EditorBlueprintResources/StandardMacros.NegateFloat` _returnvalue_2)
            (:`  `
              (`self.K2_SetActorLocation` (`KismetMathLibrary.MakeVector` _returnvalue _result) true)))))
      (if (<= _returnvalue_x_5 (`self.MinX`))
        (set `self.EnemyState` "NewEnumerator5")
        (set `self.IsRetreat` true)
        (`self.K2_SetActorRotation` (struct))
        (set `self.Speed` 1000.0)
        (if (== (`KismetMathLibrary.RandomInteger` 1) 0)
          (bind _result_2 (`/Engine/EditorBlueprintResources/StandardMacros.NegateFloat` _retreatyposition)
            (:`  `
              (`self.K2_SetActorLocation` (`KismetMathLibrary.MakeVector` _returnvalue_x_6 _result_2 _returnvalue_z) true)))
          (else
            (`self.K2_SetActorLocation` (`KismetMathLibrary.MakeVector` _returnvalue_x_6 _retreatyposition _returnvalue_z) true)))))
    (:`NewEnumerator4`
      (`GameplayStatics.SpawnEmitterAtLocation` "/Game/Realistic_Starter_VFX_Pack_Vol2/Particles/Explosion/P_Explosion_Big_A.P_Explosion_Big_A" (`self.K2_GetActorLocation`))
      (`self.K2_DestroyActor`))
    (:`NewEnumerator5`
      (`self.K2_SetActorLocation` (`KismetMathLibrary.MakeVector` (- _returnvalue_x_2 (* -1.0 (`self.Speed`) DeltaSeconds)) _returnvalue_y) true)
      (if (>= _returnvalue_x_4 5000.0)
        (`/Game/Blueprints/BP_EnemySpawner.NotifyEnemyAlived` (`self.Spawner`) self)
        (`self.K2_DestroyActor`)))))

(event `self.Box.OnComponentHit`
  (params (HitComponent :type "PrimitiveComponent Object Reference") (OtherActor :type "Actor Object Reference") (OtherComp :type "PrimitiveComponent Object Reference") (NormalImpulse :type "Vector Structure") (Hit :type "HitResult Structure (by ref)"))
  (`GameplayStatics.SpawnEmitterAtLocation` "/Game/Realistic_Starter_VFX_Pack_Vol2/Particles/Explosion/P_Explosion_Big_A.P_Explosion_Big_A" (`self.K2_GetActorLocation`) (struct) (1.0 1.0 1.0) true "None" false)
  (`/Game/Blueprints/BP_EnemySpawner.NotifyEnemyDestroyed` (`self.Spawner`) self)
  (`self.K2_DestroyActor`))

(fn `Fire`
  (if (not (`self.IsRetreat`))
    (`|ExecutionSequence`
      (:`then_0`
        (bind _returnvalue (`|SpawnActorFromClass` "/Game/Blueprints/NPC_Bullet_Child.NPC_Bullet_Child_C" (`KismetMathLibrary.MakeTransform` (`SceneComponent.K2_GetComponentLocation` (`self.BulletSpawner1`)) (`self.K2_GetActorRotation`) (0.5 0.5 0.5)) "AlwaysSpawn" "MultiplyWithRoot" null null))
        (`GameplayStatics.PlaySound2D` "/Game/Sounds/SFX/Blaster_sfx.Blaster_sfx" 1.0 1.0 0.0 null null)
        (`self.SetOwner` _returnvalue self))
      (:`then_1`
        (bind _returnvalue_2 (`|SpawnActorFromClass` "/Game/Blueprints/NPC_Bullet_Child.NPC_Bullet_Child_C" (`KismetMathLibrary.MakeTransform` (`SceneComponent.K2_GetComponentLocation` (`self.BulletSpawner2`)) (`self.K2_GetActorRotation`) (0.5 0.5 0.5)) "AlwaysSpawn" "MultiplyWithRoot" null null))
        (`GameplayStatics.PlaySound2D` "/Game/Sounds/SFX/Blaster_sfx.Blaster_sfx" 1.0 1.0 0.0 null null)
        (`self.SetOwner` _returnvalue_2 self))
      (:`then_2`
        (bind _returnvalue_3 (`|SpawnActorFromClass` "/Game/Blueprints/NPC_Bullet_Child.NPC_Bullet_Child_C" (`KismetMathLibrary.MakeTransform` (`SceneComponent.K2_GetComponentLocation` (`self.BulletSpawner3`)) (`self.K2_GetActorRotation`) (0.5 0.5 0.5)) "AlwaysSpawn" "MultiplyWithRoot" null null))
        (`GameplayStatics.PlaySound2D` "/Game/Sounds/SFX/Blaster_sfx.Blaster_sfx" 1.0 1.0 0.0 null null)
        (`self.SetOwner` _returnvalue_3 self)))))

(fn `UserConstructionScript`)