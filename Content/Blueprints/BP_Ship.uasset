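; Player-controlled ship pawn that moves on the XY plane, fires twin blasters and loses lives on collision.
; BeginPlay adds the Enhanced Input mapping context; movement actions offset the location by Speed with a swept SetActorLocation, without delta-time scaling.
; Two Fire handlers each spawn a half-scale Bullet from their own spawner and play the blaster sound.
; Box hits print a debug message, decrement Lifes and fetch HUD widgets, leaving them unused.
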(event `EnhancedInput|/Game/Inputs/RightLeft`
  (params (ActionValue :type "Float (double-precision)") (ElapsedSeconds :type "Float (double-precision)") (TriggeredSeconds :type "Float (double-precision)") (InputAction :type "InputAction Object Reference" :default "/Game/Inputs/RightLeft.RightLeft"))
  (bind (_returnvalue_x _returnvalue_y) (`KismetMathLibrary.BreakVector` (`self.K2_GetActorLocation`)))
  (:`Triggered`
    (`self.K2_SetActorLocation` (`KismetMathLibrary.MakeVector` _returnvalue_x (+ _returnvalue_y (* ActionValue (`self.Speed`)))) true)))

(event `EnhancedInput|/Game/Inputs/UpDown`
  (params (ActionValue :type "Float (double-precision)") (ElapsedSeconds :type "Float (double-precision)") (TriggeredSeconds :type "Float (double-precision)") (InputAction :type "InputAction Object Reference" :default "/Game/Inputs/UpDown.UpDown"))
  (bind (_returnvalue_x _returnvalue_y) (`KismetMathLibrary.BreakVector` (`self.K2_GetActorLocation`)))
  (:`Triggered`
    (`self.K2_SetActorLocation` (`KismetMathLibrary.MakeVector` (+ _returnvalue_x (* (`self.Speed`) ActionValue)) _returnvalue_y) true)))

(event `self.ReceiveBeginPlay`
  (bind _asplayer_controller (cast `PlayerController` (`self.GetController`)))
  (message `EnhancedInputSubsystemInterface.AddMappingContext` (pcsubsystem `EnhancedInputLocalPlayerSubsystem` _asplayer_controller) "/Game/Inputs/InputMappingContext.InputMappingContext" 0 (struct)))

(event `EnhancedInput|/Game/Inputs/Fire`
  (params (ActionValue :type Boolean) (ElapsedSeconds :type "Float (double-precision)") (TriggeredSeconds :type "Float (double-precision)") (InputAction :type "InputAction Object Reference" :default "/Game/Inputs/Fire.Fire"))
  (:`Started`
    (`|SpawnActorFromClass` "/Game/Blueprints/Bullet.Bullet_C" (`KismetMathLibrary.MakeTransform` (`SceneComponent.K2_GetComponentLocation` (`self.Spawner_Bullet_01`)) (`self.K2_GetActorRotation`) (0.5 0.5 0.5)) "Undefined" "MultiplyWithRoot" null null)
    (`GameplayStatics.PlaySound2D` "/Game/Sounds/SFX/Blaster_sfx.Blaster_sfx" 1.0 1.0 0.0 null null)))

(event `EnhancedInput|/Game/Inputs/Fire`
  (params (ActionValue :type Boolean) (ElapsedSeconds :type "Float (double-precision)") (TriggeredSeconds :type "Float (double-precision)") (InputAction :type "InputAction Object Reference" :default "/Game/Inputs/Fire.Fire"))
  (:`Started`
    (`|SpawnActorFromClass` "/Game/Blueprints/Bullet.Bullet_C" (`KismetMathLibrary.MakeTransform` (`SceneComponent.K2_GetComponentLocation` (`self.Spawner_Bullet_02`)) (`self.K2_GetActorRotation`) (0.5 0.5 0.5)) "Undefined" "MultiplyWithRoot" null null)
    (`GameplayStatics.PlaySound2D` "/Game/Sounds/SFX/Blaster_sfx.Blaster_sfx" 1.0 1.0 0.0 null null)))

(event `self.Box.OnComponentHit`
  (params (HitComponent :type "PrimitiveComponent Object Reference") (OtherActor :type "Actor Object Reference") (OtherComp :type "PrimitiveComponent Object Reference") (NormalImpulse :type "Vector Structure") (Hit :type "HitResult Structure (by ref)"))
  (`KismetSystemLibrary.PrintString` "HIT")
  (set `self.Lifes` (- (`self.Lifes`) 1))
  (`WidgetBlueprintLibrary.GetAllWidgetsOfClass` "/Game/HUD/HUD.HUD_C" false))

(fn `UserConstructionScript`)